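; BP_BattleCamera is a battle camera on a spring arm that can be set rotating around its yaw axis.
; The construction script clamps distance for the arm length, derives arm pitch from the arcsine of height over distance, and clamps the camera's own pitch.
; StartRotating and StopRotating toggle IsRotating and set or zero the RotatingMovement yaw rate.
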(event EventBeginPlay
  ;[1 1 1] Camera Settings are set in ConstructionScript
)

(fn ConstructionScript
  (Variables|CameraControls|SetCameraDistance (Math|Float|Clamp(Float) (Variables|CameraControls|GetCameraDistance) 1e+03 2e+03))
  ;[1 1 1] Set Values
  ;;[1 1 1] Set Arm Length
  (Variables|/Script/Engine.SpringArmComponent|SetTargetArmLength (Variables|Default|GetSpringArm) (Variables|CameraControls|GetCameraDistance))
  ;;[1 1 1] Set Arm Angle to get Camera Height
  (Transformation|SetRelativeRotation (Variables|Default|GetSpringArm) (Math|Rotator|MakeRotator 0.0 (Class|KismetMathLibrary|DegAsin (/ (Variables|CameraControls|GetCameraHeight) (Variables|CameraControls|GetCameraDistance))) 0.0) false false)
  ;;[1 1 1] Set Camera Angle
  (Transformation|SetRelativeRotation (Variables|Default|GetCamera) (Math|Rotator|MakeRotator 0.0 (Math|Float|ClampAngle (Variables|CameraControls|GetCameraAngle) -45.0 0.0) 0.0) false false))

(fn StartRotating
  (Variables|CameraControls|SetbIsRotating true)
  (Variables|/Script/Engine.RotatingMovementComponent|SetRotationRate (Variables|Default|GetRotatingMovement) (Math|Rotator|MakeRotator 0.0 0.0 (Variables|Default|GetZRotationRate))))

(fn StopRotating
  (Variables|CameraControls|SetbIsRotating false)
  (Variables|/Script/Engine.RotatingMovementComponent|SetRotationRate (Variables|Default|GetRotatingMovement) "0, 0, 0"))