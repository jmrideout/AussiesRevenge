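; EnemyBase is a Blueprint that tracks an enemy's health as it takes damage.
; AnyDamage subtracts damage from EnemHealth, calls CheckEnemHealth, then branches on IsDead with no action attached.
; CheckEnemHealth uses a DoOnce when health reaches zero or below, but it sets IsDead to false, so nothing here marks the enemy dead.
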(event Custom|CheckEnemHealth
  ;[1 1 1] Check Health
  ;;[1 1 1] Check IsDead
  (if (<= (Variables|Default|GetEnemHealth) 0.0)
    (Utilities|FlowControl|DoOnce false
      (:Completed
        (Variables|Default|SetIsDead false)))))

(event Game|Damage|EventAnyDamage
  (params (Damage :type Float%20%28single-precision%29) (DamageType :type Damage%20Type%20Object%20Reference) (InstigatedBy :type Controller%20Object%20Reference) (DamageCauser :type Actor%20Object%20Reference))
  ;[1 1 1] Check Health
  (Variables|Default|SetEnemHealth (- (Variables|Default|GetEnemHealth) Damage))
  (CallFunction|CheckEnemHealth)
  (if (Variables|Default|GetIsDead)
    _))

(fn ConstructionScript)